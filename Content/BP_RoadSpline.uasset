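; Road actor that lays a mesh along an editable spline, built in the construction script.
; GenerateRoad loops over the MainSpline points, adding a spline mesh component with RoadMesh that runs from each point to the next in local space.
; Segment tangents are scaled down from the spline's own, and each segment gets query and physics collision with a blocking profile.
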(fn ConstructionScript
  (CallFunction|GenerateRoad))

(fn GenerateRoad
  (bind _mainspline (Variables|Default|GetMainSpline))
  (bind _mainspline_2 (Variables|Default|GetMainSpline))
  (for _index (range 0 (- (Spline|GetNumberOfSplinePoints (Variables|Default|GetMainSpline)) 1))
    (bind _returnvalue (AddComponent|AddSplineMeshComponent false))
    (Components|StaticMesh|SetStaticMesh _returnvalue (Variables|Default|GetRoadMesh))
    (SplineMesh|SetStartandEnd _returnvalue (Spline|GetLocationatSplinePoint _mainspline _index "Local") (* (Spline|GetTangentatSplinePoint _mainspline _index "Local") 0.2) (Spline|GetLocationatSplinePoint _mainspline_2 (+ _index 1) "Local") (* (Spline|GetTangentatSplinePoint _mainspline_2 (+ _index 1) "Local") 0.2) true :!class /Script/Engine.SplineMeshComponent)
    (Collision|SetCollisionEnabled _returnvalue "QueryAndPhysics")
    (Collision|SetCollisionProfileName _returnvalue "BlockAll" true :!class /Script/Engine.PrimitiveComponent)))