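; BP_Checkpoint is a numbered checkpoint trigger that tracks the off-road car's ordered progress through a course.
; On box overlap, it advances BP_OffroadCar_Pawn only from the preceding checkpoint number, storing its number and location on the car, then calling UpdateCheckpoint.
; If the car's current checkpoint already equals its last on overlap, it instead shows WBP_Victory, pauses the game and shows the mouse cursor.
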(event OnComponentBeginOverlap(Box)
  (params (OverlappedComponent :type Primitive%20Component%20Object%20Reference) (OtherActor :type Actor%20Object%20Reference) (OtherComp :type Primitive%20Component%20Object%20Reference) (OtherBodyIndex :type Integer) (bFromSweep :type Boolean) (SweepResult :type Hit%20Result%20Structure%20%28by%20ref%29))
  (bind _asbp_offroad_car_pawn (Utilities|Casting|CastToBP_OffroadCar_Pawn OtherActor))
  (if (== (Variables|/Game/VehicleTemplate/Blueprints/OffroadCar/BP_OffroadCar_Pawn.BP_OffroadCar_Pawn_C|GetLastCheckpoint _asbp_offroad_car_pawn) (Variables|/Game/VehicleTemplate/Blueprints/OffroadCar/BP_OffroadCar_Pawn.BP_OffroadCar_Pawn_C|GetCurrentCheckpoint _asbp_offroad_car_pawn))
    (bind _returnvalue (UserInterface|CreateWidget "/Game/Blueprint/WBP_Victory.WBP_Victory_C"))
    (UserInterface|Viewport|AddtoViewport _returnvalue 0)
    (Game|SetGamePaused true)
    (Variables|/Script/Engine.PlayerController|SetbShowMouseCursor (Game|GetPlayerController 0) true)
    (elif (== (Variables|/Game/VehicleTemplate/Blueprints/OffroadCar/BP_OffroadCar_Pawn.BP_OffroadCar_Pawn_C|GetCurrentCheckpoint _asbp_offroad_car_pawn) (- (Variables|Default|GetCheckpointNumber) 1))
      (Variables|/Game/VehicleTemplate/Blueprints/OffroadCar/BP_OffroadCar_Pawn.BP_OffroadCar_Pawn_C|SetCurrentCheckpoint _asbp_offroad_car_pawn (Variables|Default|GetCheckpointNumber))
      (Variables|/Script/RunOnTheDesert.RunOnTheDesertPawn|SetcurrentCheckpointPosition _asbp_offroad_car_pawn (Transformation|GetActorLocation))
      (Default|UpdateCheckpoint _asbp_offroad_car_pawn))))

(event EventBeginPlay)

(event Collision|EventActorBeginOverlap
  (params (OtherActor :type Actor%20Object%20Reference)))

(event EventTick
  (params (DeltaSeconds :type Float%20%28single-precision%29)))

(fn ConstructionScript)